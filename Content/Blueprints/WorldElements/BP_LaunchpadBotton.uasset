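; BP_LaunchpadBotton is a world button that toggles whether its referenced Launchpad can launch.
; Action and OutOfAction events, filtered to BP_Character, enable or disable the button's input for player 0 and open or close a gate.
; Pressing the Action input while the gate is open flips the Launchpad's CanLaunch flag.
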(event EventBeginPlay)

(event Collision|EventActorBeginOverlap
  (params (OtherActor :type Actor%20Object%20Reference)))

(event EventTick
  (params (DeltaSeconds :type Float%20%28single-precision%29)))

(event EventOutOfAction
  (params (CharacterInZone :type MMM%20Character%20Object%20Reference))
  (Utilities|Casting|CastToBP_Character CharacterInZone)
  (Input|DisableInput (Game|GetPlayerController 0))
  (Utilities|FlowControl|Gate true) ; enters at Close
)

(event EventAction
  (params (CharacterInZone :type MMM%20Character%20Object%20Reference))
  (Utilities|Casting|CastToBP_Character CharacterInZone)
  (Input|EnableInput (Game|GetPlayerController 0))
  (Utilities|FlowControl|Gate true) ; enters at Open
)

(event Input|ActionEvents|InputActionAction
  (params (Key :type Key%20Structure :default "None"))
  (:Pressed
    (Utilities|FlowControl|Gate true
      (:Exit
        (if (Variables|/Game/Blueprints/WorldElements/BP_Launchpad.BP_Launchpad_C|GetbCanLaunch (Variables|Default|GetLaunchpad))
          (Variables|/Game/Blueprints/WorldElements/BP_Launchpad.BP_Launchpad_C|SetbCanLaunch (Variables|Default|GetLaunchpad) false)
          (else
            (Variables|/Game/Blueprints/WorldElements/BP_Launchpad.BP_Launchpad_C|SetbCanLaunch (Variables|Default|GetLaunchpad) true)))))))

(fn ConstructionScript)